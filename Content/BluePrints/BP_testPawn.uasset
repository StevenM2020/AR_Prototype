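; BP_testPawn is a test pawn that places objects in an AR scene on touch.
; On touch press it casts the game mode to AR_GameMode and spawns a BP_PlaceableStart at the stored ObjectCords, always spawning regardless of collisions.
; A disconnected debug chain that spawns and prints the new actor's location is never run, and the other events are empty.
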(event EventBeginPlay)

(event Collision|EventActorBeginOverlap
  (params (OtherActor :type Actor%20Object%20Reference)))

(event EventTick
  (params (DeltaSeconds :type Float%20%28single-precision%29)))

(event Input|TouchEvents|InputTouch
  (params (Location :type Vector) (FingerIndex :type ETouchIndex%20Enum)))

(event Input|TouchEvents|InputTouch
  (params (Location :type Vector) (FingerIndex :type ETouchIndex%20Enum))
  (:Pressed
    (bind _asar_game_mode (Utilities|Casting|CastToAR_GameMode (Game|GetGameMode)))
    (Game|SpawnActorfromClass "/Game/BluePrints/BP_PlaceableStart.BP_PlaceableStart_C" (Math|Conversions|ToTransform(Vector) (Variables|/Game/AR_ImageTracking/AR_GameMode.AR_GameMode_C|GetObjectCords _asar_game_mode)) "AlwaysSpawn" 0 0)))

(fn ConstructionScript)